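; Interactable cauldron that gives the player controller's active enchantment to the interacting character, with only one character enchanted at a time.
; Interacting transfers it from the previous holder, or removes it if the interactor already holds it, showing a HUD message.
; It refuses when no enchantment is active or a ghost-enchanted character is inside a wall.
; BeginPlay caches controller and game state, applies an optional test enchantment and plays a bubbling sound.
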(event EventBeginPlay
  ;[1 1 1] Begin Play
  (Utilities|FlowControl|Sequence
    (:then_0
      (bind _asbp_nolbplayer_controller (Utilities|Casting|CastToBP_NOLBPlayerController (Game|GetPlayerController 0)))
      (Variables|Internal|SetPlayer%20Controller _asbp_nolbplayer_controller)
      (if (Utilities|Enum|NotEqual(Enum) (Variables|Default|GetTest%20Enchantment) "NewEnumerator0")
        (Variables|/Game/Blueprints/GameMode/BP_NOLBPlayerController.BP_NOLBPlayerController_C|SetEnchantment%20In%20Play (Variables|Internal|GetPlayer%20Controller) (Variables|Default|GetTest%20Enchantment))))
    (:then_1
      (bind _asbp_no_one_left_behind_game_state (Utilities|Casting|CastToBP_NoOneLeftBehindGameState (Game|GetGameState)))
      (Variables|Internal|SetGame%20State _asbp_no_one_left_behind_game_state))
    (:then_2
      (Audio|PlaySoundatLocation "/Game/Audio_Files/SoundEffects/bubbling_cauldron_Cue.bubbling_cauldron_Cue" (Transformation|GetWorldLocation (Variables|Default|GetStaticMesh)) "0, 0, 0" 1.0 1.0 0.0 0 0 0 0))))

(event EventOnInteracted
  (params (Interacting%20Character :type BP%20Character%20Base%20Object%20Reference))
  (if (Utilities|Enum|NotEqual(Enum) (Variables|/Game/Blueprints/GameMode/BP_NOLBPlayerController.BP_NOLBPlayerController_C|GetEnchantment%20In%20Play (Variables|Internal|GetPlayer%20Controller)) "NewEnumerator0")
    (if (not (Variables|/Game/Blueprints/GameMode/BP_NOLBPlayerController.BP_NOLBPlayerController_C|GetCharacter%20In%20Wall (Variables|Internal|GetPlayer%20Controller)))
      (if (!= (Variables|/Game/Blueprints/GameMode/BP_NOLBPlayerController.BP_NOLBPlayerController_C|GetEnchanted%20Character (Variables|Internal|GetPlayer%20Controller)) Interacting%20Character)
        (Utilities|FlowControl|Sequence
          (:then_0
            ;[1 1 1] Disenchant an already enchanted character, if one exists. Show a display message based on whether or not a character was already enchanted.
            (Utilities|IsValid (Variables|/Game/Blueprints/GameMode/BP_NOLBPlayerController.BP_NOLBPlayerController_C|GetEnchanted%20Character (Variables|Internal|GetPlayer%20Controller))
              (:Is%20Valid
                (Default|SetCharacterEnchantment (Variables|/Game/Blueprints/GameMode/BP_NOLBPlayerController.BP_NOLBPlayerController_C|GetEnchanted%20Character (Variables|Internal|GetPlayer%20Controller)) "NewEnumerator0")
                (Default|DisplayMessage (Variables|/Game/Blueprints/GameMode/BP_NoOneLeftBehindGameState.BP_NoOneLeftBehindGameState_C|GetMessage%20Widget (Variables|Internal|GetGame%20State)) (Utilities|String|Append "The " (Utilities|String|EnumtoString (Variables|/Game/Blueprints/GameMode/BP_NOLBPlayerController.BP_NOLBPlayerController_C|GetEnchantment%20In%20Play (Variables|Internal|GetPlayer%20Controller))) " Enchantment has been transfered from " (Variables|/Game/Blueprints/Characters/BP_CharacterBase.BP_CharacterBase_C|GetCharacter%20Name (Variables|/Game/Blueprints/GameMode/BP_NOLBPlayerController.BP_NOLBPlayerController_C|GetEnchanted%20Character (Variables|Internal|GetPlayer%20Controller))) " to " (Variables|/Game/Blueprints/Characters/BP_CharacterBase.BP_CharacterBase_C|GetCharacter%20Name Interacting%20Character) "!") 4.0))
              (:Is%20Not%20Valid
                (Default|DisplayMessage (Variables|/Game/Blueprints/GameMode/BP_NoOneLeftBehindGameState.BP_NoOneLeftBehindGameState_C|GetMessage%20Widget (Variables|Internal|GetGame%20State)) (Utilities|String|Append (Variables|/Game/Blueprints/Characters/BP_CharacterBase.BP_CharacterBase_C|GetCharacter%20Name Interacting%20Character) " now has the " (Utilities|String|EnumtoString (Variables|/Game/Blueprints/GameMode/BP_NOLBPlayerController.BP_NOLBPlayerController_C|GetEnchantment%20In%20Play (Variables|Internal|GetPlayer%20Controller))) " Enchantment!") 4.0))))
          (:then_1
            ;[1 1 1] Give the interacting character their enchantment.
            (Default|SetCharacterEnchantment Interacting%20Character (Variables|/Game/Blueprints/GameMode/BP_NOLBPlayerController.BP_NOLBPlayerController_C|GetEnchantment%20In%20Play (Variables|Internal|GetPlayer%20Controller)))
            (Variables|/Game/Blueprints/GameMode/BP_NOLBPlayerController.BP_NOLBPlayerController_C|SetEnchanted%20Character (Variables|Internal|GetPlayer%20Controller) Interacting%20Character)))
        (else
          ;[1 1 1] Remove the enchantment from an already enchanted character.
          (Default|DisplayMessage (Variables|/Game/Blueprints/GameMode/BP_NoOneLeftBehindGameState.BP_NoOneLeftBehindGameState_C|GetMessage%20Widget (Variables|Internal|GetGame%20State)) (Utilities|String|Append (Variables|/Game/Blueprints/Characters/BP_CharacterBase.BP_CharacterBase_C|GetCharacter%20Name Interacting%20Character) "'s " (Utilities|String|EnumtoString (Variables|/Game/Blueprints/Characters/BP_CharacterBase.BP_CharacterBase_C|GetCurrent%20Enchantment Interacting%20Character)) " Enchantment has been removed!") 4.0)
          (Default|SetCharacterEnchantment Interacting%20Character "NewEnumerator0")
          (Variables|/Game/Blueprints/GameMode/BP_NOLBPlayerController.BP_NOLBPlayerController_C|SetEnchanted%20Character (Variables|Internal|GetPlayer%20Controller) 0)))
      (else
        (Default|DisplayMessage (Variables|/Game/Blueprints/GameMode/BP_NoOneLeftBehindGameState.BP_NoOneLeftBehindGameState_C|GetMessage%20Widget (Variables|Internal|GetGame%20State)) "Someone with the Ghost Enchantment is in a wall! Move them first!" 4.0)))
    (else
      (Default|DisplayMessage (Variables|/Game/Blueprints/GameMode/BP_NoOneLeftBehindGameState.BP_NoOneLeftBehindGameState_C|GetMessage%20Widget (Variables|Internal|GetGame%20State)) "There's nothing in here! Find some ingredients and activate an enchantment!" 4.0))))

(fn ConstructionScript
  (Utilities|Array|Add (Variables|/Game/MarkObjectSystem/Component/BP_MarkObjectsComponent.BP_MarkObjectsComponent_C|GetMeshes%20To%20Mark (Variables|Default|GetBP_MarkObjectsComponent)) (Variables|Default|GetStaticMesh)))