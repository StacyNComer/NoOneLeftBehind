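; BP_PlayerMessage is an interactable that shows dialogue to a character, either on interaction or automatically at start.
; ShowMessage has the target character display InteractMessages as multi-page dialogue when there are several entries, otherwise the first entry as a single dialogue.
; With ShowOnBeginPlay set, Tick sends the message once to the first BP_CharacterBase found, then clears the flag.
; The construction script registers the static mesh with BPMarkObjectsComponent for marking.
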(event EventTick
  (params (DeltaSeconds :type Float%20%28single-precision%29))
  (if (Variables|Parameters|GetShow%20On%20Begin%20Play)
    (bind _returnvalue (Actor|GetActorOfClass "/Game/Blueprints/Characters/BP_CharacterBase.BP_CharacterBase_C"))
    (CallFunction|ShowMessage _returnvalue)
    (Variables|Parameters|SetShow%20On%20Begin%20Play false)))

(event EventOnInteracted
  (params (Interacting%20Character :type BP%20Character%20Base%20Object%20Reference))
  (CallFunction|ShowMessage Interacting%20Character))

(fn ConstructionScript
  (Utilities|Array|Add (Variables|/Game/MarkObjectSystem/Component/BP_MarkObjectsComponent.BP_MarkObjectsComponent_C|GetMeshes%20To%20Mark (Variables|Default|GetBP_MarkObjectsComponent)) (Variables|Default|GetStaticMesh)))

(fn ShowMessage
  (params (Target%20Character :type BP%20Character%20Base%20Object%20Reference))
  (if (> (Utilities|Array|Length (Variables|Parameters|GetInteract%20Messages)) 1)
    (Default|DisplayMulti-PageDialogue Target%20Character (Variables|Parameters|GetInteract%20Messages))
    (else
      (Default|DisplayDialogue Target%20Character (Utilities|Array|Get(acopy) (Variables|Parameters|GetInteract%20Messages)) 0.0))))