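; BP_Witch is a swappable playable character who toggles flight with a mid-air Jump and refuses to pick up actors.
; Flight uses custom movement mode 1: Tick follows camera-boom yaw and sweeps her along the camera's forward vector, scaled by boost or brake inputs.
; Unless braking, collisions end flight; non-walkable surfaces without the NoWitchBounce physical material bounce her back and briefly disable movement.
; Swapping characters mid-flight drops her into falling with her flight velocity.
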(event EventTick
  (params (DeltaSeconds :type Float%20%28single-precision%29))
  (bind _charactermovement (Variables|Character|GetCharacterMovement))
  (bind _returnvalue (Class|CharacterMovementComponent|GetWalkableFloorAngle _charactermovement))
  ;[1 1 1] Tick
  (|CallParentFunction DeltaSeconds)
  ;;[1 1 1] Movement while the player is flying.
  (if (CallFunction|IsFlying)
    (Transformation|SetActorRotation (Math|Rotator|MakeRotator 0.0 0.0 (.yaw (Class|SpringArmComponent|GetTargetRotation (Variables|Default|GetCameraBoom)))))
    (bind _sweephitresult (Transformation|SetActorLocation (+ (* (CallFunction|GetFlightVelocity) DeltaSeconds) (Transformation|GetActorLocation)) true false))
    (if (and (.bblockinghit _sweephitresult) (>= (Variables|Flying|GetFlight%20Speed%20Boost) 0))
      ;;;[1 1 1] The Witches flight ends if she collides with anything unless she is braking. If she hits a wall/ceiling (i.e. a surface sloped great than the max walkable angle), she gets booped backwards unless the actor has the NoWitchBounce Physics Material
      (Pawn|Components|CharacterMovement|SetMovementMode (Variables|Character|GetCharacterMovement) "MOVE_Falling" 0)
      (if (and (or (< (Class|KismetMathLibrary|DegAcos (Math|Vector|DotProduct (Math|Vector|VectorUp) (.normal _sweephitresult))) (* _returnvalue -1.0)) (> (Class|KismetMathLibrary|DegAcos (Math|Vector|DotProduct (Math|Vector|VectorUp) (.normal _sweephitresult))) _returnvalue)) (!= (.physmat _sweephitresult) "/Game/Blueprints/Misc/NoWitchBounce.NoWitchBounce"))
        (Variables|/Script/Engine.MovementComponent|SetVelocity (Variables|Character|GetCharacterMovement) (* (CallFunction|GetFlightVelocity) (Variables|Flying|GetFlight%20Bounce%20Percent) (Class|KismetSystemLibrary|MakeLiteralInteger -1)))
        (Variables|Default|SetCan%20Move? false)
        (Utilities|FlowControl|Delay 0.5)
        (Variables|Default|SetCan%20Move? true)))))

(event EventPickupActor
  (params (Liftable%20Actor :type BP%20Liftable%20Base%20Object%20Reference))
  (Default|DisplayMessage (Variables|/Game/Blueprints/GameMode/BP_NoOneLeftBehindGameState.BP_NoOneLeftBehindGameState_C|GetMessage%20Widget (Variables|Default|GetGame%20State)) "This is no job for an old lady!" 3.0))

(event EventOnCharacterSwapped
  (|CallParentFunction)
  (if (CallFunction|IsFlying)
    (Pawn|Components|CharacterMovement|SetMovementMode (Variables|Character|GetCharacterMovement) "MOVE_Falling" 0)
    (Variables|/Script/Engine.MovementComponent|SetVelocity (Variables|Character|GetCharacterMovement) (CallFunction|GetFlightVelocity))))

(event Input|ActionEvents|InputActionJump
  (params (Key :type Key%20Structure))
  (:Pressed
    (if (and (not (Character|CanJump)) (Variables|Default|GetCan%20Move?))
      (Variables|/Script/Engine.MovementComponent|SetVelocity (Variables|Character|GetCharacterMovement) (Math|Vector|SelectVector (CallFunction|GetFlightVelocity) "0, 0, 0" (CallFunction|IsFlying)))
      (Pawn|Components|CharacterMovement|SetMovementMode (Variables|Character|GetCharacterMovement) (select (CallFunction|IsFlying) "MOVE_Falling" "MOVE_Custom") 1))))

(event Input|ActionEvents|InputActionWitchFlightBoost
  (params (Key :type Key%20Structure))
  ;[1 1 1] Witch Flight Boost
  (:Pressed
    (Variables|Flying|SetFlight%20Speed%20Boost 1))
  (:Released
    (if (> (Variables|Flying|GetFlight%20Speed%20Boost) 0)
      (Variables|Flying|SetFlight%20Speed%20Boost 0))))

(event Input|ActionEvents|InputActionWitchFlightBrake
  (params (Key :type Key%20Structure))
  ;[1 1 1] Witch Flight Brake
  (:Pressed
    (Variables|Flying|SetFlight%20Speed%20Boost -1))
  (:Released
    (if (< (Variables|Flying|GetFlight%20Speed%20Boost) 0)
      (Variables|Flying|SetFlight%20Speed%20Boost 0))))

(fn ConstructionScript
  (|CallParentFunction))

(fn IsFlying
  (return (== (Variables|/Script/Engine.CharacterMovementComponent|GetCustomMovementMode (Variables|Character|GetCharacterMovement)) 1)))

(fn GetFlightVelocity
  (return (* (Math|Vector|GetForwardVector (Variables|Default|GetFollowCamera)) (Variables|/Script/Engine.CharacterMovementComponent|GetMaxCustomMovementSpeed (Variables|Character|GetCharacterMovement)) (Math|Float|SelectFloat 1.0 (Math|Float|SelectFloat (Variables|Flying|GetFlight%20Thrust%20Multiplier) (Variables|Flying|GetFlight%20%20Brake%20Multiplier) (> (Variables|Flying|GetFlight%20Speed%20Boost) 0)) (== (Variables|Flying|GetFlight%20Speed%20Boost) 0)))))