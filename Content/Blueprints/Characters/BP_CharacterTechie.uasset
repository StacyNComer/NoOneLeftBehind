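; Techie character Blueprint that replaces the parent's throw with a kinesis move, levitating a held actor out to grab range.
; While Use is held, movement is disabled and charge sweeps the actor toward KinesisEndpoint until blocked.
; Release past the threshold drops it in place with zeroed velocity; shorter presses toss it with drop force.
; The endpoint follows control yaw except during a throw, and EndThrow restores walking.
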(event EventBeginPlay
  (|CallParentFunction) ; This node is disabled and will not be called.\nDrag off pins to build functionality.
)

(event Collision|EventActorBeginOverlap
  (params (OtherActor :type Actor%20Object%20Reference)))

(event EventTick
  (params (DeltaSeconds :type Float%20%28single-precision%29))
  (|CallParentFunction DeltaSeconds)
  (if (Variables|Default|GetIs%20Throwing?)
    (CallFunction|ChargeThrow DeltaSeconds)
    (else
      (Transformation|SetWorldRotation (Variables|Default|GetKinesis%20Endpoint%20Rotation) (Math|Rotator|MakeRotator 0.0 0.0 (.yaw (Pawn|GetControlRotation :!class /Script/Engine.Pawn))) false false))))

(event Input|ActionEvents|InputActionUse
  (params (Key :type Key%20Structure :default "None"))
  (:Released
    ;[1 1 1] Throwing
    (if (Variables|Default|GetIs%20Throwing?)
      (if (> (Variables|Default|GetThrow%20Charge) (Variables|Default|GetDrop%20Charge%20Threshold))
        (CallFunction|ChargedThrow)
        (else
          (CallFunction|ThrowHeldActor (Variables|Default|GetDrop%20Force) 2e+02)))
      (CallFunction|EndThrow))))

(fn ConstructionScript
  (bind _kinesis_endpoint (Variables|Default|GetKinesis%20Endpoint))
  (|CallParentFunction)
  ;[1 1 1] Sets the transform of the kinesis endpoint so that it is always at the Techie's grab range
  (Transformation|SetRelativeLocation _kinesis_endpoint (Math|Vector|MakeVector (Variables|Default|GetGrab%20Range) 0.0 (.z (Variables|/Script/Engine.SceneComponent|GetRelativeLocation _kinesis_endpoint))) false false))

(fn ChargeThrow
  (params (Delta%20Seconds :type Float%20%28double-precision%29))
  (Variables|Default|SetThrow%20Charge (Math|Float|Min(Float) (+ Delta%20Seconds (Variables|Default|GetThrow%20Charge)) (Variables|Default|GetMax%20Throw%20Charge)))
  ;[1 1 1] Levitate the held actor forwaed until it hits something
  (if (not (Variables|Default|GetKinesis%20Hit))
    (bind _sweephitresult (Transformation|SetActorLocation (Variables|Default|GetActor%20Held) (Math|Vector|Lerp(Vector) (Transformation|GetWorldLocation (Variables|Default|GetLiftable%20Attach%20Point)) (Transformation|GetWorldLocation (Variables|Default|GetKinesis%20Endpoint)) (Math|Float|MapRangeClamped (Variables|Default|GetThrow%20Charge) (Variables|Default|GetDrop%20Charge%20Threshold) (Variables|Default|GetMax%20Throw%20Charge) 0.0 1.0)) true false))
    (Variables|Default|SetKinesis%20Hit (.bblockinghit _sweephitresult))))

(fn ChargedThrow
  (Physics|SetPhysicsLinearVelocity (Variables|/Game/Blueprints/Liftable/BP_LiftableBase.BP_LiftableBase_C|GetMesh (Variables|Default|GetActor%20Held)) "0, 0, 0" false "None")
  (CallFunction|ThrowHeldActor 0.0 0.0))

(fn ThrowPressed
  (Collision|SetCollisionEnabled (Variables|/Game/Blueprints/Liftable/BP_LiftableBase.BP_LiftableBase_C|GetMesh (Variables|Default|GetActor%20Held)) "QueryAndPhysics")
  (Pawn|Components|CharacterMovement|DisableMovement (Variables|Character|GetCharacterMovement))
  (Variables|Default|SetIs%20Throwing? true))

(fn EndThrow
  (Utilities|FlowControl|Sequence
    (:then_0
      ;[1 1 1] Drop any crates that were being levitated forward.
      (if (and (> (Variables|Default|GetThrow%20Charge) (Variables|Default|GetDrop%20Charge%20Threshold)) (Utilities|IsValid (Variables|Default|GetActor%20Held)))
        (CallFunction|ChargedThrow)))
    (:then_1
      (|CallParentFunction)
      (Variables|Default|SetKinesis%20Hit false)
      (Pawn|Components|CharacterMovement|SetMovementMode (Variables|Character|GetCharacterMovement) "MOVE_Walking" 0))))