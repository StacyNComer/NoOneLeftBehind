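; BP_LevelLoadBoundry is an interactable airlock that swaps between previous and next streamed sublevels once the required characters stand inside.
; Overlaps track occupants; interaction checks their count against characters in play or an override, showing dialogue if unmet.
; It removes characters from game state, broadcasts loading dispatchers around delayed, blocking unload/load calls, then fires load triggers and toggled plates.
; Finally it resets the controller's enchantment system and flips direction.
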(event EventOnInteracted
  (params (Interacting%20Character :type BP%20Character%20Base%20Object%20Reference))
  (bind _required_character_override (Variables|Parameters|GetRequired%20Character%20Override))
  (if (Variables|Internal|GetIsInteractable)
    (if (== (Utilities|Array|Length (Variables|Internal|GetCharacter's%20In%20Boundary)) (Math|Integer|SelectInt _required_character_override (Default|GetNumCharactersinPlay (Variables|Internal|GetGame%20State)) (> _required_character_override 0)))
      (CallFunction|SetAirlockInteractable true)
      (Default|RemoveCharacters (Variables|Internal|GetGame%20State) (Variables|Internal|GetCharacter's%20In%20Boundary))
      (Default|CallDispatcheronBeginLoading (Variables|Internal|GetLoad%20Next%20Area?))
      (Utilities|FlowControl|Delay (Variables|Parameters|GetLoad%20Delay))
      (Default|CleanRemovedCharacters (Variables|Internal|GetGame%20State))
      (Class|GameplayStatics|UnloadStreamLevelbySoftObjectPtr (select (Variables|Internal|GetLoad%20Next%20Area?) (Variables|Parameters|GetPrev%20Sublevel) (Variables|Parameters|GetNext%20Sublevel)) true)
      (Class|GameplayStatics|LoadStreamLevelbySoftObjectPtr (select (Variables|Internal|GetLoad%20Next%20Area?) (Variables|Parameters|GetNext%20Sublevel) (Variables|Parameters|GetPrev%20Sublevel)) true true)
      (Default|CallDispatcheronFinishLoading (Variables|Internal|GetLoad%20Next%20Area?))
      (Utilities|FlowControl|Sequence
        (:then_0
          (bind _outactors (Actor|GetAllActorsOfClass "/Game/Blueprints/TriggeredObjects/BP_TriggeredActorBase.BP_TriggeredActorBase_C"))
          (for _array_element _outactors
            (if (CallFunction|GetShouldTriggeronLoad (Variables|/Game/Blueprints/TriggeredObjects/BP_TriggeredActorBase.BP_TriggeredActorBase_C|GetTrigger%20On%20Load? _array_element))
              (Default|Trigger _array_element))))
        (:then_1
          (if (Variables|Internal|GetLoad%20Next%20Area?)
            (for _array_element_2 (Variables|Parameters|GetTrigger%20On%20Next%20Loaded)
              (Default|Trigger _array_element_2))
            (else
              (for _array_element_3 (Variables|Parameters|GetTrigger%20On%20Prev%20Loaded)
                (Default|Trigger _array_element_3)))))
        (:then_2
          (bind _outactors_2 (Actor|GetAllActorsOfClass "/Game/Blueprints/Switches/BP_PressurePlateToggled.BP_PressurePlateToggled_C"))
          (for _array_element_4 _outactors_2
            (if (CallFunction|GetShouldTriggeronLoad (Variables|/Game/Blueprints/Switches/BP_PressurePlateToggled.BP_PressurePlateToggled_C|GetStart%20Toggled%20On%20Load? _array_element_4))
              (Default|ForceWasTriggered _array_element_4))))
        (:then_3
          (Default|ResetEnchantmentSystem (Variables|Internal|GetPlayer%20Conroller)))
        (:then_4
          (Variables|Internal|SetLoad%20Next%20Area? (not (Variables|Internal|GetLoad%20Next%20Area?)))
          (CallFunction|SetAirlockInteractable true)))
      (else
        (Default|DisplayDialogue Interacting%20Character "All characters must be in the exit area to proceed! Leave no one behind!" 3.0)))))

(event EventBeginPlay
  (bind _asbp_no_one_left_behind_game_state (Utilities|Casting|CastToBP_NoOneLeftBehindGameState (Game|GetGameState)))
  (Variables|Internal|SetGame%20State _asbp_no_one_left_behind_game_state)
  (bind _asbp_nolbplayer_controller (Utilities|Casting|CastToBP_NOLBPlayerController (Game|GetPlayerController 0)))
  (Variables|Internal|SetPlayer%20Conroller _asbp_nolbplayer_controller))

(event Collision|EventActorBeginOverlap
  (params (OtherActor :type Actor%20Object%20Reference))
  (bind _asbp_character_base (Utilities|Casting|CastToBP_CharacterBase OtherActor))
  (Utilities|Array|Add (Variables|Internal|GetCharacter's%20In%20Boundary) _asbp_character_base))

(event Collision|EventActorEndOverlap
  (params (OtherActor :type Actor%20Object%20Reference))
  (bind _asbp_character_base (Utilities|Casting|CastToBP_CharacterBase OtherActor))
  (Utilities|Array|RemoveItem (Variables|Internal|GetCharacter's%20In%20Boundary) _asbp_character_base))

(fn ConstructionScript)

(fn GetShouldTriggeronLoad
  (params (Load%20Trigger%20Type :type ELoadTriggerType%20Enum :default "NewEnumerator0"))
  (bind _load_next_area_ (Variables|Internal|GetLoad%20Next%20Area?))
  (return (or (and (Utilities|Enum|Equal(Enum) Load%20Trigger%20Type "NewEnumerator1") _load_next_area_) (and (Utilities|Enum|Equal(Enum) Load%20Trigger%20Type "NewEnumerator2") (not _load_next_area_)))))

(fn SetAirlockInteractable
  (params (IsInteractable :type Boolean))
  (bind _bp_markobjectscomponent (Variables|Default|GetBP_MarkObjectsComponent))
  (bind _output_get (Variables|Internal|SetIsInteractable IsInteractable))
  (bind _output_get_2 (Variables|/Game/MarkObjectSystem/Component/BP_MarkObjectsComponent.BP_MarkObjectsComponent_C|SetPlayer%20Markable _bp_markobjectscomponent _output_get))
  (if (not _output_get_2)
    (Default|UnmarkObejct _bp_markobjectscomponent)))