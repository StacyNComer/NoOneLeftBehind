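; Airlock that swaps two BP_Door doors and their collision as neighboring sublevels begin and finish loading.
; It binds to begin and finish loading dispatchers, using a next-sublevel flag to choose which door to trigger or untrigger and which collision to toggle.
; The construction script casts the child-actor doors, applies a NoWitchBounce physical material and registers their meshes for marking.
; The EntranceDoor component is stored as ExitDoorActor, and vice versa.
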(event Custom|Close%20Airlock
  (params (Next%20Sublevel%20Loading? :type Boolean))
  (if Next%20Sublevel%20Loading?
    (Default|Trigger (Variables|Internal|GetExit%20Door%20Actor))
    (Collision|SetCollisionEnabled (Variables|Default|GetExit%20Door%20Collision) "NoCollision")
    (else
      (Default|Untrigger (Variables|Internal|GetEntrance%20Door%20Actor))
      (Collision|SetCollisionEnabled (Variables|Default|GetEntrance%20Door%20Collision) "NoCollision"))))

(event Custom|Open%20Airlock
  (params (Next%20Sublevel%20Loaded? :type Boolean))
  (if Next%20Sublevel%20Loaded?
    (Default|Trigger (Variables|Internal|GetEntrance%20Door%20Actor))
    (Collision|SetCollisionEnabled (Variables|Default|GetEntrance%20Door%20Collision) "QueryOnly")
    (else
      (Default|Untrigger (Variables|Internal|GetExit%20Door%20Actor))
      (Collision|SetCollisionEnabled (Variables|Default|GetExit%20Door%20Collision) "QueryOnly"))))

(event EventBeginPlay
  (|CallParentFunction)
  (EventDispatchers|AssignDispatcheronBeginLoading (delegate Custom|Close%20Airlock))
  (EventDispatchers|AssignDispatcheronFinishLoading (delegate Custom|Open%20Airlock)))

(fn ConstructionScript
  (|CallParentFunction)
  (bind _door_actor (CallFunction|InitializeDoor (Variables|Default|GetEntrance%20Door)))
  (Variables|Internal|SetExit%20Door%20Actor _door_actor)
  (bind _door_actor_2 (CallFunction|InitializeDoor (Variables|Default|GetExit%20Door)))
  (Variables|Internal|SetEntrance%20Door%20Actor _door_actor_2))

(fn InitializeDoor
  (params (Door%20Child%20Component :type Child%20Actor%20Component%20Object%20Reference))
  (bind _asbp_door (Utilities|Casting|CastToBP_Door (Variables|/Script/Engine.ChildActorComponent|GetChildActor Door%20Child%20Component)))
  (bind _output_get (LocalVariables|SetCasted%20Door _asbp_door))
  (Class|PrimitiveComponent|SetPhysMaterialOverride (Variables|/Game/Blueprints/TriggeredObjects/BP_MovingPlatform.BP_MovingPlatform_C|GetMesh _output_get) "/Game/Blueprints/Misc/NoWitchBounce.NoWitchBounce")
  (Utilities|Array|Add (Variables|/Game/MarkObjectSystem/Component/BP_MarkObjectsComponent.BP_MarkObjectsComponent_C|GetMeshes%20To%20Mark (Variables|Default|GetBP_MarkObjectsComponent)) (Variables|/Game/Blueprints/TriggeredObjects/BP_MovingPlatform.BP_MovingPlatform_C|GetMesh _output_get))
  (return (LocalVariables|GetCasted%20Door)))