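; BP_SecretOrb is a collectable that marks a found secret in the game.
; On BeginPlay it binds GrabSecret to the OnCollectedDispatch event dispatcher.
; GrabSecret increments SecretsCollected on BP_NoOneLeftBehindGameState and has the collector display a short congratulatory dialogue, skipping both if the game state cast fails.
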(event Custom|Grab%20Secret
  (params (Collector :type BP%20Character%20Base%20Object%20Reference))
  (bind _asbp_no_one_left_behind_game_state (Utilities|Casting|CastToBP_NoOneLeftBehindGameState (Game|GetGameState)))
  (Math|Integer|IncrementInt (Variables|/Game/Blueprints/GameMode/BP_NoOneLeftBehindGameState.BP_NoOneLeftBehindGameState_C|GetSecrets%20Collected _asbp_no_one_left_behind_game_state)
    (:%20%20
      (Default|DisplayDialogue Collector "Nice! You've found a secret!" 3.0))))

(event EventBeginPlay
  (|CallParentFunction)
  (EventDispatchers|AssignOnCollectedDispatch (delegate Custom|Grab%20Secret)))

(event Collision|EventActorBeginOverlap
  (params (OtherActor :type Actor%20Object%20Reference))
  (|CallParentFunction OtherActor) ; This node is disabled and will not be called.\nDrag off pins to build functionality.
)

(event EventTick
  (params (DeltaSeconds :type Float%20%28single-precision%29))
  (|CallParentFunction DeltaSeconds) ; This node is disabled and will not be called.\nDrag off pins to build functionality.
)

(fn ConstructionScript
  (|CallParentFunction))